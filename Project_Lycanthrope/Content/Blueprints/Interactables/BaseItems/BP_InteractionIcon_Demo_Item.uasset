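; BP_InteractionIcon_Demo_Item is a demo interactable that shows proximity-based interaction indicators to the player.
; Two nested trigger spheres toggle an outer and an inner visual, responding only to player character 0.
; Entering the outer sphere shows the outer visual, and leaving hides it.
; Entering the inner sphere swaps to the inner visual, and leaving swaps back to the outer one.
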(event `self.SC_InnerSphere.OnComponentBeginOverlap`
  (params (OverlappedComponent :type "PrimitiveComponent Object Reference") (OtherActor :type "Actor Object Reference") (OtherComp :type "PrimitiveComponent Object Reference") (OtherBodyIndex :type Integer) (bFromSweep :type Boolean) (SweepResult :type "HitResult Structure (by ref)"))
  (if (== OtherActor (`GameplayStatics.GetPlayerCharacter` 0))
    (`SceneComponent.SetVisibility` (`self.B_OuterSphere`) false false)
    (`SceneComponent.SetVisibility` (`self.B_InnerSpere`) true false)))

(event `self.SC_InnerSphere.OnComponentEndOverlap`
  (params (OverlappedComponent :type "PrimitiveComponent Object Reference") (OtherActor :type "Actor Object Reference") (OtherComp :type "PrimitiveComponent Object Reference") (OtherBodyIndex :type Integer))
  (if (== (`GameplayStatics.GetPlayerCharacter` 0) OtherActor)
    (`SceneComponent.SetVisibility` (`self.B_OuterSphere`) true false)
    (`SceneComponent.SetVisibility` (`self.B_InnerSpere`) false false)))

(event `self.SC_OuterSphere.OnComponentBeginOverlap`
  (params (OverlappedComponent :type "PrimitiveComponent Object Reference") (OtherActor :type "Actor Object Reference") (OtherComp :type "PrimitiveComponent Object Reference") (OtherBodyIndex :type Integer) (bFromSweep :type Boolean) (SweepResult :type "HitResult Structure (by ref)"))
  (if (== OtherActor (`GameplayStatics.GetPlayerCharacter` 0))
    (`SceneComponent.SetVisibility` (`self.B_OuterSphere`) true false)))

(event `self.SC_OuterSphere.OnComponentEndOverlap`
  (params (OverlappedComponent :type "PrimitiveComponent Object Reference") (OtherActor :type "Actor Object Reference") (OtherComp :type "PrimitiveComponent Object Reference") (OtherBodyIndex :type Integer))
  (if (== (`GameplayStatics.GetPlayerCharacter` 0) OtherActor)
    (`SceneComponent.SetVisibility` (`self.B_OuterSphere`) false false)))

(fn `UserConstructionScript`)