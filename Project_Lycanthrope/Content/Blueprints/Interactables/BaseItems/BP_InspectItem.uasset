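; Item inspection actor that shows a supplied mesh with an item info or readable note widget.
; Inspect and ReadNote switch input from the player character to this actor, with setters for starting rotation and scale.
; Mouse and look input rotate the mesh, while wheel and gamepad stick adjust SceneCapture FOV to zoom, all gated by InNote.
; Jump toggles note text visibility; Interact restores player input, removing widgets and destroying the actor when the inspect widget exists.
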(event `Key|RightMouseButton`
  (params (Key :type "Key Structure"))
  ;[0.03 0.03 0.2 0.5] Rotation Check
  (:`Pressed`
    (set `self.rotate?` true))
  (:`Released`
    (set `self.rotate?` false)))

(event `/Game/Blueprints/Interface/BPI_Interaction.Read Note`
  (params (Character :type "/Game/ThirdPerson/Blueprints/BP_ThirdPersonCharacter Object Reference") (`Note Text` :type Text))
  (bind _returnvalue (`GameplayStatics.GetPlayerController` 0))
  ;[0.03 0.03 0.2 0.5] Read Note
  (set `self.Character` Character)
  (bind _returnvalue_2 (`|CreateWidget` "/Game/Blueprints/Interactables/Widgets/WB_Note.WB_Note_C" null `Note Text`))
  (bind _output_get (set `self.Note Widget Ref` _returnvalue_2))
  (`UserWidget.AddToViewport` _output_get 0)
  (`Widget.SetRenderOpacity` (`/Game/Blueprints/Interactables/Widgets/WB_Note.B_Read` (`self.Note Widget Ref`)) 1.0)
  (`self.DisableInput` (`GameplayStatics.GetPlayerCharacter` 0) _returnvalue)
  (`self.EnableInput` _returnvalue))

(event `InputAxisKey|MouseX`
  (params (AxisValue :type "Float (single-precision)"))
  ;[0.03 0.03 0.2 0.5] set mouse movement horiziontal
  (if (not (`self.InNote?`))
    (if (`self.rotate?`)
      (`SceneComponent.K2_SetWorldRotation` (`self.SM_Item`) (`KismetMathLibrary.ComposeRotators` (`SceneComponent.K2_GetComponentRotation` (`self.SM_Item`)) (`KismetMathLibrary.MakeRotator` 0.0 0.0 (* AxisValue -3.0))) false false))))

(event `/Game/Blueprints/Interface/BPI_Interaction.Inspect`
  (params (Character :type "/Game/ThirdPerson/Blueprints/BP_ThirdPersonCharacter Object Reference") (`Inspected  Item` :type "StaticMesh Object Reference") (`Item Name` :type Text) (`Item Description` :type Text))
  (bind _returnvalue (`GameplayStatics.GetPlayerController` 0))
  ;[0.03 0.03 0.2 0.5] Inspect Item (Dynamically getting Inspect info)
  (set `self.Character` Character)
  (`StaticMeshComponent.SetStaticMesh` (`self.SM_Item`) `Inspected  Item`)
  (bind _returnvalue_2 (`|CreateWidget` "/Game/Blueprints/Interactables/Widgets/WB_inspect.WB_inspect_C" null `Item Name` `Item Description`))
  (bind _output_get (set `self.InspectWidget Ref` _returnvalue_2))
  (`UserWidget.AddToViewport` _output_get 0)
  (`self.DisableInput` (`GameplayStatics.GetPlayerCharacter` 0) _returnvalue)
  (`self.EnableInput` _returnvalue)
  (set `self.InNote?` false))

(event `InputAxisKey|MouseY`
  (params (AxisValue :type "Float (single-precision)"))
  ;[0.03 0.03 0.2 0.5] set mouse movement vertically
  (if (not (`self.InNote?`))
    (if (`self.rotate?`)
      (`SceneComponent.K2_SetWorldRotation` (`self.SM_Item`) (`KismetMathLibrary.ComposeRotators` (`SceneComponent.K2_GetComponentRotation` (`self.SM_Item`)) (`KismetMathLibrary.MakeRotator` 0.0 (* AxisValue -3.0))) false false))))

(event `EnhancedInput|/Game/Input/Actions/IA_interact`
  (params (ActionValue :type Boolean) (ElapsedSeconds :type "Float (double-precision)") (TriggeredSeconds :type "Float (double-precision)") (InputAction :type "InputAction Object Reference" :default "/Game/Input/Actions/IA_interact.IA_interact"))
  (bind _returnvalue (`GameplayStatics.GetPlayerController` 0))
  (bind _inspectwidget_ref (`self.InspectWidget Ref`))
  (bind _note_widget_ref (`self.Note Widget Ref`))
  ;[0.03 0.03 0.2 0.5] Destorying actor after exiting view
  (:`Started`
    (`self.DisableInput` _returnvalue)
    (`self.EnableInput` (`GameplayStatics.GetPlayerCharacter` 0) _returnvalue)
    (`/Engine/EditorBlueprintResources/StandardMacros.IsValid` _inspectwidget_ref
      (:`Is Valid`
        (`Widget.RemoveFromParent` _inspectwidget_ref)
        (set `self.InspectWidget Ref` null)
        (`self.K2_DestroyActor`)
        (`/Engine/EditorBlueprintResources/StandardMacros.IsValid` _note_widget_ref
          (:`Is Valid`
            (`Widget.RemoveFromParent` _note_widget_ref)
            (set `self.Note Widget Ref` null)
            (`self.K2_DestroyActor`)))))))

(event `Key|MouseScrollUp`
  (params (Key :type "Key Structure"))
  (bind _scenecapturecomponent2d (`self.SceneCaptureComponent2D`))
  ;[0.03 0.03 0.2 0.5] Zoom In
  (:`Pressed`
    (if (not (`self.InNote?`))
      (set `SceneCaptureComponent2D.FOVAngle` (`KismetMathLibrary.FClamp` (- (`SceneCaptureComponent2D.FOVAngle` _scenecapturecomponent2d) 1.0) 40.0 80.0) _scenecapturecomponent2d))))

(event `Set Inspect Rotation`
  (params (`Item Rotation` :type "Rotator Structure"))
  (bind (_returnvalue_location _returnvalue_rotation _returnvalue_scale) (`KismetMathLibrary.BreakTransform` (`SceneComponent.K2_GetComponentToWorld` (`self.SM_Item`))))
  ;[0.03 0.03 0.2 0.5] Setting Inspect Rotation
  (bind _output_get (set `self.Intitial Item Rotation` `Item Rotation`))
  (`SceneComponent.K2_SetWorldTransform` (`self.SM_Item`) (`KismetMathLibrary.MakeTransform` _returnvalue_location _output_get _returnvalue_scale) false false))

(event `EnhancedInput|/Game/Input/Actions/IA_Jump`
  (params (ActionValue :type Boolean) (ElapsedSeconds :type "Float (double-precision)") (TriggeredSeconds :type "Float (double-precision)") (InputAction :type "InputAction Object Reference" :default "/Game/Input/Actions/IA_Jump.IA_Jump"))
  ;[0.03 0.03 0.2 0.5] Pressed key To Read
  (:`Started`
    (bind _isa (`/Engine/EditorBlueprintResources/StandardMacros.FlipFlop`)
      (:`A`
        (set `self.Is A` _isa)
        (`Widget.SetRenderOpacity` (`/Game/Blueprints/Interactables/Widgets/WB_Note.CP_Note` (`self.Note Widget Ref`)) 1.0)
        (set `self.Is A` false)
        (set `self.InNote?` true))
      (:`B`
        (`Widget.SetRenderOpacity` (`/Game/Blueprints/Interactables/Widgets/WB_Note.CP_Note` (`self.Note Widget Ref`)) 0.0)
        (set `self.Is A` false)))))

(event `Key|Gamepad_LeftStick_Up`
  (params (Key :type "Key Structure"))
  (bind _scenecapturecomponent2d (`self.SceneCaptureComponent2D`))
  ;[0.03 0.03 0.2 0.5] Zoom In
  (:`Pressed`
    (if (not (`self.InNote?`))
      (set `SceneCaptureComponent2D.FOVAngle` (`KismetMathLibrary.FClamp` (- (`SceneCaptureComponent2D.FOVAngle` _scenecapturecomponent2d) 5.0) 40.0 80.0) _scenecapturecomponent2d))))

(event `Set Inspect Scale`
  (params (`Item Scale` :type "Vector Structure"))
  (bind (_returnvalue_location _returnvalue_rotation) (`KismetMathLibrary.BreakTransform` (`SceneComponent.K2_GetComponentToWorld` (`self.SM_Item`))))
  ;[0.03 0.03 0.2 0.5] Setting Inspect Scale
  (`SceneComponent.K2_SetWorldTransform` (`self.SM_Item`) (`KismetMathLibrary.MakeTransform` _returnvalue_location _returnvalue_rotation `Item Scale`) false false))

(event `Key|MouseScrollDown`
  (params (Key :type "Key Structure"))
  (bind _scenecapturecomponent2d (`self.SceneCaptureComponent2D`))
  ;[0.03 0.03 0.2 0.5] Zoom Out
  (:`Pressed`
    (if (not (`self.InNote?`))
      (set `SceneCaptureComponent2D.FOVAngle` (`KismetMathLibrary.FClamp` (+ (`SceneCaptureComponent2D.FOVAngle` _scenecapturecomponent2d) 1.0) 40.0 80.0) _scenecapturecomponent2d))))

(event `Key|Gamepad_LeftStick_Down`
  (params (Key :type "Key Structure"))
  (bind _scenecapturecomponent2d (`self.SceneCaptureComponent2D`))
  ;[0.03 0.03 0.2 0.5] Zoom Out
  (:`Pressed`
    (if (not (`self.InNote?`))
      (set `SceneCaptureComponent2D.FOVAngle` (`KismetMathLibrary.FClamp` (+ (`SceneCaptureComponent2D.FOVAngle` _scenecapturecomponent2d) 5.0) 40.0 80.0) _scenecapturecomponent2d))))

(event `EnhancedInput|/Game/Input/Actions/IA_Look`
  (params (ActionValue :type "Vector2D Structure") (ElapsedSeconds :type "Float (double-precision)") (TriggeredSeconds :type "Float (double-precision)") (InputAction :type "InputAction Object Reference" :default "/Game/Input/Actions/IA_Look.IA_Look"))
  ;[0.03 0.03 0.2 0.5] W A S D Movement
  (:`Triggered`
    (if (not (`self.InNote?`))
      (if (or (!= ActionValue_X 0.0) (!= ActionValue_Y 0.0))
        (`|ExecutionSequence`
          (:`then_0`
            (`SceneComponent.K2_SetWorldRotation` (`self.SM_Item`) (`KismetMathLibrary.ComposeRotators` (`SceneComponent.K2_GetComponentRotation` (`self.SM_Item`)) (`KismetMathLibrary.MakeRotator` 0.0 0.0 (* ActionValue_X -2.0))) false false))
          (:`then_1`
            (`SceneComponent.K2_SetWorldRotation` (`self.SM_Item`) (`KismetMathLibrary.ComposeRotators` (`SceneComponent.K2_GetComponentRotation` (`self.SM_Item`)) (`KismetMathLibrary.MakeRotator` 0.0 (* ActionValue_Y -2.0))) false false)))))))

(fn `UserConstructionScript`)