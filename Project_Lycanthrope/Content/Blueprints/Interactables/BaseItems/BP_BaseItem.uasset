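; Base interactable item actor that shows proximity icons and can open an inspection view of its mesh.
; Outer and inner sphere overlaps with the player swap two icons, and the outer one also toggles the crosshair widget.
; On interaction, if inspection is enabled, it spawns a far-off BP_InspectItem and passes it the mesh, name, description, rotation and scale.
; The construction script applies mesh, scale, icon location and debug visibility.
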(event `self.SC_InnerSphere.OnComponentBeginOverlap`
  (params (OverlappedComponent :type "PrimitiveComponent Object Reference") (OtherActor :type "Actor Object Reference") (OtherComp :type "PrimitiveComponent Object Reference") (OtherBodyIndex :type Integer) (bFromSweep :type Boolean) (SweepResult :type "HitResult Structure (by ref)"))
  ;[0.03 0.03 0.2 0.5] Icons
  ;;[0.03 0.03 0.2 0.5] Setting Inner Sphere Icon
  (if (== OtherActor (`GameplayStatics.GetPlayerCharacter` 0))
    (`SceneComponent.SetVisibility` (`self.B_OuterSphere`) false false)
    (`SceneComponent.SetVisibility` (`self.B_InnerSpere`) true false)))

(event `self.SC_InnerSphere.OnComponentEndOverlap`
  (params (OverlappedComponent :type "PrimitiveComponent Object Reference") (OtherActor :type "Actor Object Reference") (OtherComp :type "PrimitiveComponent Object Reference") (OtherBodyIndex :type Integer))
  ;[0.03 0.03 0.2 0.5] Icons
  ;;[0.03 0.03 0.2 0.5] Setting Inner Sphere Icon
  (if (== (`GameplayStatics.GetPlayerCharacter` 0) OtherActor)
    (`SceneComponent.SetVisibility` (`self.B_OuterSphere`) true false)
    (`SceneComponent.SetVisibility` (`self.B_InnerSpere`) false false)))

(event `self.SC_OuterSphere.OnComponentBeginOverlap`
  (params (OverlappedComponent :type "PrimitiveComponent Object Reference") (OtherActor :type "Actor Object Reference") (OtherComp :type "PrimitiveComponent Object Reference") (OtherBodyIndex :type Integer) (bFromSweep :type Boolean) (SweepResult :type "HitResult Structure (by ref)"))
  ;[0.03 0.03 0.2 0.5] Icons
  ;;[0.03 0.03 0.2 0.5] Setting Outer sphere icon and Dynamic Crosshair
  (if (== OtherActor (`GameplayStatics.GetPlayerCharacter` 0))
    (`SceneComponent.SetVisibility` (`self.B_OuterSphere`) true false)
    (bind _foundwidgets (`WidgetBlueprintLibrary.GetAllWidgetsOfClass` "/Game/HUD/MainUI/WB_Crosshair.WB_Crosshair_C"))
    (`Widget.SetVisibility` _foundwidgets "Visible")))

(event `self.SC_OuterSphere.OnComponentEndOverlap`
  (params (OverlappedComponent :type "PrimitiveComponent Object Reference") (OtherActor :type "Actor Object Reference") (OtherComp :type "PrimitiveComponent Object Reference") (OtherBodyIndex :type Integer))
  ;[0.03 0.03 0.2 0.5] Icons
  ;;[0.03 0.03 0.2 0.5] Setting Outer sphere icon and Dynamic Crosshair
  (if (== (`GameplayStatics.GetPlayerCharacter` 0) OtherActor)
    (`SceneComponent.SetVisibility` (`self.B_OuterSphere`) false false)
    (bind _foundwidgets (`WidgetBlueprintLibrary.GetAllWidgetsOfClass` "/Game/HUD/MainUI/WB_Crosshair.WB_Crosshair_C"))
    (`Widget.SetVisibility` _foundwidgets "Hidden")))

(event `/Game/Blueprints/Interface/BPI_Interaction.Interaction`
  (params (character :type "/Game/ThirdPerson/Blueprints/BP_ThirdPersonCharacter Object Reference"))
  ;[0.03 0.03 0.2 0.5] Item Inspecion
  (if (`self.Inspect?`)
    (bind _returnvalue (`|SpawnActorFromClass` "/Game/Blueprints/Interactables/BaseItems/BP_InspectItem.BP_InspectItem_C" (`KismetMathLibrary.MakeTransform` (100000000000.0 0.0 0.0)) "Undefined" "MultiplyWithRoot" null null))
    (`/Game/Blueprints/Interactables/BaseItems/BP_InspectItem.Set Inspect Rotation` _returnvalue (`self.Item Inspection Rotation`))
    (`/Game/Blueprints/Interactables/BaseItems/BP_InspectItem.Set Inspect Scale` _returnvalue (`self.Item inspection Scale`))
    (message `/Game/Blueprints/Interface/BPI_Interaction.Inspect` _returnvalue character (`StaticMeshComponent.StaticMesh` (`self.SM_Item`)) (`self.Item Name`) (`self.Item Description`))))

(fn `UserConstructionScript`
  (bind _sm_item (`self.SM_Item`))
  (`|ExecutionSequence`
    (:`then_0`
      ;[0.03 0.03 0.2 0.5] Setting Icon location
      (`SceneComponent.K2_SetRelativeLocation` (`self.B_InnerSpere`) (`self.Icon Location`) false false)
      (`SceneComponent.K2_SetRelativeLocation` (`self.B_OuterSphere`) (`self.Icon Location`) false false))
    (:`then_1`
      ;[0.03 0.03 0.2 0.5] Dynamically setting mesh
      (`StaticMeshComponent.SetStaticMesh` (`self.SM_Item`) (`self.Item Mesh`))
      ;[0.03 0.03 0.2 0.5] Setting Item scale
      (`SceneComponent.K2_SetWorldTransform` _sm_item (`KismetMathLibrary.MakeTransform` (`SceneComponent.K2_GetComponentLocation` _sm_item) (`SceneComponent.K2_GetComponentRotation` _sm_item) (`self.Item Scale`)) false false))
    (:`then_2`
      ;[0.03 0.03 0.2 0.5] Check if in debug mode
      (if (`self.Debugging?`)
        (`SceneComponent.SetVisibility` (`self.SC_OuterSphere`) true false)
        (`SceneComponent.SetVisibility` (`self.SC_InnerSphere`) true false)
        (`SceneComponent.SetVisibility` (`self.B_OuterSphere`) true false)
        (`SceneComponent.SetVisibility` (`self.B_InnerSpere`) true false)
        (else
          (`SceneComponent.SetVisibility` (`self.SC_OuterSphere`) false false)
          (`SceneComponent.SetVisibility` (`self.SC_InnerSphere`) false false)
          (`SceneComponent.SetVisibility` (`self.B_OuterSphere`) false false)
          (`SceneComponent.SetVisibility` (`self.B_InnerSpere`) false false))))))