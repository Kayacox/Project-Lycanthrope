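; Interactable item actor that shows proximity icons and toggles the crosshair as the player approaches.
; Entering the outer sphere shows the outer icon and any top-level WB_Crosshair widgets; leaving it hides both.
; The inner sphere swaps the outer icon for the inner one while the player overlaps it, and restores it on exit.
; The Interaction event is a placeholder that only prints a debug string.
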(event `self.Interaction`
  (`KismetSystemLibrary.PrintString` "Interacted" true true (struct :`R` 0.03 :`G` 0.2 :`B` 0.03 :`A` 1.0)))

(event `self.SC_InnerSphere.OnComponentBeginOverlap`
  (params (OverlappedComponent :type "PrimitiveComponent Object Reference") (OtherActor :type "Actor Object Reference") (OtherComp :type "PrimitiveComponent Object Reference") (OtherBodyIndex :type Integer) (bFromSweep :type Boolean) (SweepResult :type "HitResult Structure (by ref)"))
  ;[0.03 0.03 0.2 0.5] Icons
  ;;[0.03 0.03 0.2 0.5] Setting Inner Sphere Icon
  (if (== OtherActor (`GameplayStatics.GetPlayerCharacter` 0))
    (`SceneComponent.SetVisibility` (`self.B_OuterSphere`) false false)
    (`SceneComponent.SetVisibility` (`self.B_InnerSpere`) true false)))

(event `self.SC_InnerSphere.OnComponentEndOverlap`
  (params (OverlappedComponent :type "PrimitiveComponent Object Reference") (OtherActor :type "Actor Object Reference") (OtherComp :type "PrimitiveComponent Object Reference") (OtherBodyIndex :type Integer))
  ;[0.03 0.03 0.2 0.5] Icons
  ;;[0.03 0.03 0.2 0.5] Setting Inner Sphere Icon
  (if (== (`GameplayStatics.GetPlayerCharacter` 0) OtherActor)
    (`SceneComponent.SetVisibility` (`self.B_OuterSphere`) true false)
    (`SceneComponent.SetVisibility` (`self.B_InnerSpere`) false false)))

(event `self.SC_OuterSphere.OnComponentBeginOverlap`
  (params (OverlappedComponent :type "PrimitiveComponent Object Reference") (OtherActor :type "Actor Object Reference") (OtherComp :type "PrimitiveComponent Object Reference") (OtherBodyIndex :type Integer) (bFromSweep :type Boolean) (SweepResult :type "HitResult Structure (by ref)"))
  ;[0.03 0.03 0.2 0.5] Icons
  ;;[0.03 0.03 0.2 0.5] Setting Outer sphere icon and Dynamic Crosshair
  (if (== OtherActor (`GameplayStatics.GetPlayerCharacter` 0))
    (`SceneComponent.SetVisibility` (`self.B_OuterSphere`) true false)
    (bind _foundwidgets (`WidgetBlueprintLibrary.GetAllWidgetsOfClass` "/Game/HUD/MainUI/WB_Crosshair.WB_Crosshair_C"))
    (`Widget.SetVisibility` _foundwidgets "Visible")))

(event `self.SC_OuterSphere.OnComponentEndOverlap`
  (params (OverlappedComponent :type "PrimitiveComponent Object Reference") (OtherActor :type "Actor Object Reference") (OtherComp :type "PrimitiveComponent Object Reference") (OtherBodyIndex :type Integer))
  ;[0.03 0.03 0.2 0.5] Icons
  ;;[0.03 0.03 0.2 0.5] Setting Outer sphere icon and Dynamic Crosshair
  (if (== (`GameplayStatics.GetPlayerCharacter` 0) OtherActor)
    (`SceneComponent.SetVisibility` (`self.B_OuterSphere`) false false)
    (bind _foundwidgets (`WidgetBlueprintLibrary.GetAllWidgetsOfClass` "/Game/HUD/MainUI/WB_Crosshair.WB_Crosshair_C"))
    (`Widget.SetVisibility` _foundwidgets "Hidden")))

(fn `UserConstructionScript`)